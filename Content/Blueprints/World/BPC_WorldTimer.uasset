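; World timer Blueprint component that turns elapsed game time into an in-game clock and drives the day-night lighting.
; UpdateTimer splits game seconds by a configurable day length into day, hour, minute and second, then derives a sun angle.
; UpdateLight pitches the sun, refreshes the sky sphere and blends skylight cubemaps from dusk toward night or noon using the angle's sine.
; BeginPlay and Tick are unused.
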(event Custom|UpdateLight
  (params (LightDirection :type Float%20%28single-precision%29))
  (bind _returnvalue (Math|Trig|Sin(Degrees) LightDirection))
  (bind _skylight (Variables|Default|GetSkyLight))
  (bind _returnvalue_2 (Math|Float|Absolute(Float) _returnvalue))
  (bind _lightcomponent (Variables|/Script/Engine.SkyLight|GetLightComponent _skylight))
  (Transformation|SetActorRelativeRotation (Variables|Default|GetSunLight) (Math|Rotator|MakeRotator 0.0 LightDirection 0.0))
  (Default|UpdateSunDirection (Variables|Default|GetSkySphere))
  (if (>= _returnvalue 0.0)
    (Class|SkyLightComponent|SetCubemapBlend _lightcomponent "/Game/Textures/Render/RT_Dusk.RT_Dusk" "/Game/Textures/Render/RT_Night.RT_Night" _returnvalue_2)
    (else
      (Class|SkyLightComponent|SetCubemapBlend _lightcomponent "/Game/Textures/Render/RT_Dusk.RT_Dusk" "/Game/Textures/Render/RT_Noon.RT_Noon" _returnvalue_2))))

(event EventBeginPlay)

(event EventTick
  (params (DeltaSeconds :type Float%20%28single-precision%29)))

(event EventUpdateTimer
  (bind _returnvalue (Utilities|Time|GetTimeSeconds))
  (bind _secondsofday (Variables|Default|GetSecondsOfDay))
  (bind (_remainder _returnvalue_2) (Math|Float|Division(WholeandRemainder) _returnvalue _secondsofday))
  (bind _returnvalue_3 (/ _secondsofday 24.0))
  (bind (_remainder_2 _returnvalue_4) (Math|Float|Division(WholeandRemainder) _remainder _returnvalue_3))
  (bind _returnvalue_5 (/ _returnvalue_3 6e+01))
  (bind (_remainder_3 _returnvalue_6) (Math|Float|Division(WholeandRemainder) _remainder_2 _returnvalue_5))
  (Utilities|FlowControl|Sequence
    (:then_0
      (Variables|Default|SetTimeSeconds (Math|Float|Truncate _returnvalue))
      (Variables|Default|SetCurrentDay _returnvalue_2)
      (Variables|Default|SetCurrentHour _returnvalue_4)
      (Variables|Default|SetCurrentMinute _returnvalue_6)
      (Variables|Default|SetCurrentSeconds (.ReturnValue (Math|Float|Division(WholeandRemainder) _remainder_3 (/ _returnvalue_5 6e+01)))))
    (:then_1
      (CallFunction|UpdateLight (+ (* (/ (/ _remainder _returnvalue_3) 24.0) 3.6e+02) 2e+02)))))