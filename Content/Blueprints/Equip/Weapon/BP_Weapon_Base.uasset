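; Base weapon Blueprint that reports valid hits to its owning character through the Gameplay Ability System.
; When OnHitTarget fires, it ignores the owner and accepts only actors derived from DWCharacter or VitalityObject.
; It then sends an Event.Hit.Attack gameplay event to the owner, with the owner as instigator and the hit actor as target.
; The Blueprint applies no damage itself.
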(event EventBeginPlay)

(event Collision|EventActorBeginOverlap
  (params (OtherActor :type Actor%20Object%20Reference)))

(event EventTick
  (params (DeltaSeconds :type Float%20%28single-precision%29)))

(event EventOnHitTarget
  (params (OverlappedComponent :type Primitive%20Component%20Object%20Reference) (OtherActor :type Actor%20Object%20Reference) (OtherComp :type Primitive%20Component%20Object%20Reference) (OtherBodyIndex :type Integer) (bFromSweep :type Boolean) (SweepResult :type Hit%20Result%20Structure%20%28by%20ref%29))
  (bind _returnvalue (Utilities|GetClass OtherActor))
  (if (and (!= OtherActor (Variables|Default|GetOwnerCharacter)) (or (Utilities|ClassIsChildOf _returnvalue "/Script/DreamWorld.DWCharacter") (Utilities|ClassIsChildOf _returnvalue "/Script/DreamWorld.VitalityObject")))
    (Ability|SendGameplayEventtoActor (Variables|Default|GetOwnerCharacter) "(TagName=\"Event.Hit.Attack\")" (Utilities|Struct|MakeGameplayEventData "" (Variables|Default|GetOwnerCharacter) OtherActor))))

(fn ConstructionScript)