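; Base Blueprint for remote skill actors that report hits on characters and vitality objects back to their owner.
; OnHitTarget ignores the owner; for DWCharacter or VitalityObject targets it plays an impact sound and particle effect at the skill's location.
; It then sends an Event.Hit.Skill gameplay event to the owner with instigator and target, leaving any further effect to the receiver.
; The actor destroys itself on any non-owner hit.
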(event EventBeginPlay)

(event Collision|EventActorBeginOverlap
  (params (OtherActor :type Actor%20Object%20Reference)))

(event EventTick
  (params (DeltaSeconds :type Float%20%28single-precision%29)))

(event EventOnHitTarget
  (params (OverlappedComponent :type Primitive%20Component%20Object%20Reference) (OtherActor :type Actor%20Object%20Reference) (OtherComp :type Primitive%20Component%20Object%20Reference) (OtherBodyIndex :type Integer) (bFromSweep :type Boolean) (SweepResult :type Hit%20Result%20Structure%20%28by%20ref%29))
  (bind _returnvalue (Utilities|GetClass OtherActor))
  (bind _returnvalue_2 (Transformation|GetActorLocation))
  (if (!= OtherActor (Variables|Default|GetOwnerCharacter))
    (if (or (Utilities|ClassIsChildOf _returnvalue "/Script/DreamWorld.DWCharacter") (Utilities|ClassIsChildOf _returnvalue "/Script/DreamWorld.VitalityObject"))
      (Audio|PlaySoundatLocation "/Game/Sounds/Stab_Tone03.Stab_Tone03" _returnvalue_2 "0, 0, 0" 1.0 1.0 0.0 0 0 0)
      (Effects|SpawnEmitteratLocation "/Game/Effects/Particle_Systems/P_Impact_WeaponDamage.P_Impact_WeaponDamage" _returnvalue_2)
      (Ability|SendGameplayEventtoActor (Variables|Default|GetOwnerCharacter) "(TagName=\"Event.Hit.Skill\")" (Utilities|Struct|MakeGameplayEventData "" (Variables|Default|GetOwnerCharacter) OtherActor))
      (Actor|DestroyActor)
      (else
        (Actor|DestroyActor)))))

(fn ConstructionScript)