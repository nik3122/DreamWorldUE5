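; Base Blueprint for human characters, providing a visibility toggle and a cape that animates with the body.
; The construction script sets the body mesh as the Cape's master pose component, so the cape follows its animation.
; SetVisible propagates visibility from the capsule to all children, then re-hides BigDecal and MeshHighlight when showing, so those overlays stay off.
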(event EventSetVisible
  (params (bVisible :type Boolean))
  (Rendering|SetVisibility (Variables|Default|GetCapsuleComponent) bVisible true)
  (if bVisible
    (Rendering|SetVisibility (Variables|Default|GetBigDecal) false false)
    (Rendering|SetVisibility (Variables|Default|GetMesh%20highlight) false false)))

(fn ConstructionScript
  (Class|SkinnedMeshComponent|SetMasterPoseComponent (Variables|Default|GetCape) (Variables|Character|GetMesh) false) ; Set cape mesh to match animations of player mesh
)